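; BP_Door is an interactive door that the player swings open and shut with the E key while standing in its trigger box.
; Box overlap with BP_ThirdPersonCharacter enables input on the door, and leaving the box disables it.
; A FlipFlop on E alternates playing and reversing a timeline whose float track drives the yaw of MainDoor's relative rotation.
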(event OnComponentBeginOverlap(Box)
  (params (OverlappedComponent :type Primitive%20Component%20Object%20Reference) (OtherActor :type Actor%20Object%20Reference) (OtherComp :type Primitive%20Component%20Object%20Reference) (OtherBodyIndex :type Integer) (bFromSweep :type Boolean) (SweepResult :type Hit%20Result%20Structure%20%28by%20ref%29))
  ;[0.3073 0.3073 0.3073] Enables/Disables the Input if player in zone
  (Utilities|Casting|CastToBP_ThirdPersonCharacter OtherActor)
  (Input|EnableInput (Game|GetPlayerController 0)))

(event OnComponentEndOverlap(Box)
  (params (OverlappedComponent :type Primitive%20Component%20Object%20Reference) (OtherActor :type Actor%20Object%20Reference) (OtherComp :type Primitive%20Component%20Object%20Reference) (OtherBodyIndex :type Integer))
  ;[0.3073 0.3073 0.3073] Enables/Disables the Input if player in zone
  (Utilities|Casting|CastToBP_ThirdPersonCharacter OtherActor)
  (Input|DisableInput (Game|GetPlayerController 0) 0))

(event Input|KeyboardEvents|E
  (params (Key :type Key%20Structure))
  ;[0.4792 0.4792 0.4792 1 10] When Key pressed it do the animation with Timeline & takes the door variable To set the Relative rotation also 'Make Rotator is used to take new rotaion value
  (:Pressed
    (Utilities|FlowControl|FlipFlop
      (:A
        (bind _newtrack_1 (Timeline|Door%20Rotaion%20Time PlayFromStart)
          (:Update
            (Transformation|SetRelativeRotation (Variables|Default|GetMainDoor) (Math|Rotator|MakeRotator 0.0 0.0 _newtrack_1) false false))))
      (:B
        (Timeline|Door%20Rotaion%20Time ReverseFromEnd)))))

(fn ConstructionScript)